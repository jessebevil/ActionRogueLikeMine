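; BP_TreasureChest is an interactable chest that responds only to a pawn holding the required key card.
; On Interact, it looks for an exact match of the RequiredKeyCard gameplay tag among the instigator's SActionComponent active tags.
; A timeline then pitches the lid, and on finishing activates the particle system and starts a second CloseLid timeline on the same lid rotation.
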(event EventInteract
  (params (InstigatorPawn :type Pawn%20Object%20Reference))
  (bind _lidmesh (Variables|Default|GetLidMesh))
  (if (GameplayTags|HasTag (Variables|/Script/ActionRogueLikeMine.SActionComponent|GetActiveGameplayTags (Actor|GetComponentbyClass InstigatorPawn "/Script/ActionRogueLikeMine.SActionComponent")) (Variables|Default|GetRequired%20KeyCard) true)
    (bind _pitch (Timeline|Animate%20Lid Play)
      (:Update
        (Transformation|SetRelativeRotation _lidmesh (Math|Rotator|MakeRotator 0.0 _pitch 0.0) false false))
      (:Finished
        (Components|Activation|Activate (Variables|Default|GetParticleSystem) false)
        (bind _pitch_2 (Timeline|CloseLid Play)
          (:Update
            (Transformation|SetRelativeRotation _lidmesh (Math|Rotator|MakeRotator 0.0 _pitch_2 0.0) false false)))))))

(fn ConstructionScript)