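; Interactable lever that toggles its handle between up and down and triggers another actor when switched on.
; Each Interact alternates through a FlipFlop, setting the handle mesh's relative rotation.
; Activation also sends InteractMessage to SelectedActor with the instigating pawn and adds a KeyCard gameplay tag to that pawn's SActionComponent active tags.
; Deactivation only rotates the handle, leaving the target and tag untouched.
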(event EventInteract
  (params (InstigatorPawn :type Pawn%20Object%20Reference))
  (Utilities|FlowControl|FlipFlop
    (:A
      (Transformation|SetRelativeRotation (Variables|Default|GetHandle_Mesh) (|HandleUp(Activate)) false false)
      (Class|SGameplayInterface|Interact(Message) (Variables|Default|GetSelected%20Actor) InstigatorPawn)
      (GameplayTags|AddGameplayTag (Variables|/Script/ActionRogueLikeMine.SActionComponent|GetActiveGameplayTags (Actor|GetComponentbyClass InstigatorPawn "/Script/ActionRogueLikeMine.SActionComponent")) (Variables|Default|GetKeyCard) :!class /Script/GameplayTags.BlueprintGameplayTagLibrary))
    (:B
      (Transformation|SetRelativeRotation (Variables|Default|GetHandle_Mesh) (|HandleDown(Deactivate)) false false))))

(fn ConstructionScript)